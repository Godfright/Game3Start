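; BP_EnemyBase is an enemy character that moves toward the player on BeginPlay using AI MoveTo.
; Attack plays a zombie attack montage and calls OnAttackEnd whether it completes or is interrupted.
; SpawnFire spawns a BP_Fire actor and attaches it to a hand socket on the mesh.
; ExtinguishFire calls SpawnFire again, then destroys an actor.
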(event `self.ReceiveBeginPlay`
  (`|AIMoveTo` self (0.0 0.0 0.0) (`GameplayStatics.GetPlayerCharacter` 0) 200.0))

(event `Attack`
  (`|PlayMontage` (`self.Mesh`) "/Game/Content/BSP_ZombieAnims/Animations/Standing/Attack/AS_NAAT_Zombie_Attack_RH_Stand_Montage.AS_NAAT_Zombie_Attack_RH_Stand_Montage"
    (:`OnCompleted`
      _)
    (:`OnInterrupted`
      _))
  (`self.OnAttackEnd`))

(event `SpawnFire`
  (bind _returnvalue (`|SpawnActorFromClass` "/Game/Blueprints/BP_Fire.BP_Fire_C" (`SceneComponent.K2_GetComponentToWorld` (`self.CapsuleComponent`)) "Undefined" "MultiplyWithRoot" null null))
  (`self.K2_AttachToComponent` _returnvalue (`self.Mesh`) "hand_rFire" "KeepRelative" "KeepRelative" "KeepRelative" true))

(event `ExtinguishFire`
  (`self.SpawnFire`)
  (`self.K2_DestroyActor`))

(fn `UserConstructionScript`)