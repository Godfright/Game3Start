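; Projectile bullet-drop test actor that draws a hand-written trajectory simulation alongside Unreal's built-in projectile path prediction.
; BeginPlay repeats both every 1.5 seconds from the Arrow's location.
; BigBallzDrop line-traces up to SimFrequency debug-drawn segments, stopping on a hit, then resets start and velocity.
; Its steps divide only X velocity by SimFrequency, folding time scaling for Z into gravity (-980/SimFrequency²).
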(event `BigBallzDrop`
  (set `self.End` (+ (`self.Start`) (/ (`self.Velocity`) (`KismetMathLibrary.MakeVector` (`self.SimFrequency`) 1.0 1.0))))
  (for _ (range 1 (+ (`KismetMathLibrary.FTrunc` (`self.SimFrequency`)) 1))
    (`KismetSystemLibrary.DrawDebugLine` (`self.Start`) (`self.End`) (struct :`R` 0.673586 :`G` 0.027282 :`B` 1.0 :`A` 1.0) (`self.MaxSimTime`))
    (`KismetSystemLibrary.DrawDebugSphere` (`self.End`) 5.0 12 (struct :`R` 0.121782 :`G` 0.673505 :`B` 1.0 :`A` 1.0) (`self.MaxSimTime`))
    (bind (_outhit _returnvalue) (`KismetSystemLibrary.LineTraceSingleByProfile` :`Start` (`self.Start`) :`End` (`self.End`) :`ProfileName` "BlockAll" :`DrawDebugType` "ForDuration"))
    (if _returnvalue
      (`KismetSystemLibrary.PrintString` "ITS A HIT" true true (struct :`R` 1.0 :`B` 0.004 :`A` 1.0))
      (break)
      (else
        (`KismetSystemLibrary.PrintString` "DID NOT hit" true true (struct :`R` 1.0 :`G` 0.005604 :`B` 0.383549 :`A` 1.0))
        (set `self.Start` (`self.End`)) ; set the NEW start location
        (set `self.Velocity` (+ (`self.Velocity`) (`KismetMathLibrary.MakeVector` 0.0 0.0 (/ -980.0 (`KismetMathLibrary.Square` (`self.SimFrequency`))))))
        (set `self.End` (+ (`self.Start`) (/ (`self.Velocity`) (`KismetMathLibrary.MakeVector` (`self.SimFrequency`) 1.0 1.0)))))))
  ;[1 1 1] Reset start and velocity
  (set `self.Start` (`SceneComponent.K2_GetComponentLocation` (`self.Arrow`)))
  (set `self.Velocity` (`self.StartingVelocity`)))

(event `self.ReceiveBeginPlay`
  (set `self.End` (+ (`self.Start`) (/ (`self.Velocity`) (`KismetMathLibrary.MakeVector` (`self.SimFrequency`) 1.0 1.0))))
  (set `self.Start` (`SceneComponent.K2_GetComponentLocation` (`self.Arrow`)))
  (`|ExecutionSequence` :!label _label
    (:`then_0`
      (`GameplayStatics.Blueprint_PredictProjectilePath_Advanced` (make `PredictProjectilePathParams` (`self.Start`) (`self.StartingVelocity`) true 0.0 (`self.MaxSimTime`) true "ECC_WorldStatic" _ _ (`self.SimFrequency`) 0.0 "ForDuration"))
      (`KismetSystemLibrary.Delay` 1.5)
      (goto _label))
    (:`then_1`
      (`self.BigBallzDrop`))))

(fn `UserConstructionScript`)