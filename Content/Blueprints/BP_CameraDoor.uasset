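; BP_CameraDoor is a door actor that can briefly take over the player camera when triggered.
; OpenDoor, gated on Closed, records the door in GM_2Coding's LevelSAVE open-door list, blends the view to itself, then back to the passed target after a short delay.
; A separate quietOpen event slides the mesh down via a timeline and sets Closed true when finished.
; OpenDoor itself neither moves the door nor calls quietOpen.
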(event `quietOpen`
  (bind (_direction _newtrack_0) (`Timeline|Timeline`)
    (:`Update`
      (`SceneComponent.K2_SetRelativeLocation` (`self.Door`) (`KismetMathLibrary.VLerp` (0.0 0.0 150.0) (0.0 0.0 -130.0) _newtrack_0) false false))
    (:`Finished`
      (set `self.Closed` true))))

(event `OpenDoor`
  (params (NewViewTarget :type "Actor Object Reference"))
  (if (`self.Closed`)
    (bind _asgm_2coding (cast `/Game/Blueprints/NewSaves/GM_2Coding` (`GameplayStatics.GetGameMode`)))
    (`KismetArrayLibrary.Array_AddUnique` (`/Game/Blueprints/NewSaves/SG_LevelSAVE.NEWOpenDoors` (`/Game/Blueprints/NewSaves/GM_2Coding.LevelSAVE` _asgm_2coding)) self)
    (`PlayerController.SetViewTargetWithBlend` (`GameplayStatics.GetPlayerController` 0) self (`self.Blend Time`) "VTBlend_Cubic" 0.0 true)
    (`KismetSystemLibrary.Delay` 0.2) ; waiting 2 seconds while the door opens
    (`PlayerController.SetViewTargetWithBlend` (`GameplayStatics.GetPlayerController` 0) NewViewTarget (/ (`self.Blend Time`) 2.0) "VTBlend_Cubic" 0.0 false) ; shift camera back to player
  ))

(fn `UserConstructionScript`)