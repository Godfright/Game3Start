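; Dialogue system Blueprint that automatically plays through the lines in DT_Dialogues on screen, with debug prints.
; Shortly after BeginPlay it creates the W_DataTableDialogue widget, then DebugSystem fetches rows by index to set the text.
; Each row's speaker selects a UV Location on the portrait's dynamic material to switch faces.
; DebugSystem re-calls itself after a fixed delay to advance while rows are found, without player input.
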(event `self.ReceiveBeginPlay`
  (`KismetSystemLibrary.Delay` 2.0)
  (bind _returnvalue (`|CreateWidget` "/Game/Blueprints/Widgets/W_DataTableDialogue.W_DataTableDialogue_C"))
  (bind _output_get (set `self.W_Dialogue` _returnvalue))
  (`UserWidget.AddToViewport` _output_get 0)
  (`self.DebugSystem`))

(event `DebugSystem`
  (`KismetSystemLibrary.PrintString` "Starting debug system")
  (bind _outrownames (`DataTableFunctionLibrary.GetDataTableRowNames` "/Game/Blueprints/DataTables/DT_Dialogues.DT_Dialogues"))
  (bind _returnvalue (`|GetDataTableRow` "/Game/Blueprints/DataTables/DT_Dialogues.DT_Dialogues" (`|GetArrayItem` _outrownames (`self.RowIndex`)))
    (:`then`
      (`TextBlock.SetText` (`/Game/Blueprints/Widgets/W_DataTableDialogue.TextBlock_0` (stale `self.ReceiveBeginPlay` _output_get)) (break `/Game/Blueprints/Structures/S_DialogueLines` _returnvalue))
      (bind _image_0 (`/Game/Blueprints/Widgets/W_DataTableDialogue.Image_0` (stale `self.ReceiveBeginPlay` _output_get)))
      (bind _returnvalue_2 (`Image.GetDynamicMaterial` _image_0))
      (`Image.SetBrushFromMaterial` _image_0 _returnvalue_2)
      (bind (_returnvalue_x _returnvalue_y) (`KismetMathLibrary.BreakVector` (select `/Game/Blueprints/Enumerations/E_Character` (`.Speaker_12_DF8C92F6448E7BDA1B71588F62BF5AE1` (break `/Game/Blueprints/Structures/S_DialogueLines` _returnvalue)) :`NewEnumerator1` (0.0 1.0 0.0) :`NewEnumerator2` (0.0 2.0 0.0) :!type "Vector Structure")))
      ;[1 1 1] Change the image of who is talking
      (`MaterialInstanceDynamic.SetVectorParameterValue` _returnvalue_2 "UV Location" (make `LinearColor` _returnvalue_x _returnvalue_y 0.0 1.0))
      (`KismetSystemLibrary.PrintString` "Vector parameter set")
      (`KismetSystemLibrary.Delay` 2.0)
      ;[1 1 1] Go to next line
      (`/Engine/EditorBlueprintResources/StandardMacros.IncrementInt` (`self.RowIndex`)
        (:`  `
          (`self.DebugSystem`))))))

(fn `UserConstructionScript`)