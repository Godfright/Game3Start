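; BP_Weapon is a weapon Blueprint with a weapon type, an elemental type and a damage range, shown on three text elements.
; RandomizeValues adds a small random bump to MinDamage, derives MaxDamage from it with another random offset, then calls UpdateText.
; UpdateText writes both enum names and the min-max range, with TextWeaponType receiving the elemental type and TextElemType the weapon type.
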(event `RandomizeValues`
  (bind _output_get (set `self.MinDamage` (+ (`self.MinDamage`) (`KismetMathLibrary.RandomInteger` 2))))
  (set `self.MaxDamage` (+ _output_get (`KismetMathLibrary.RandomIntegerInRange` 1)))
  (`self.UpdateText`))

(event `UpdateText`
  (`TextRenderComponent.K2_SetText` (`self.TextWeaponType`) (`KismetTextLibrary.Conv_StringToText` (`|GetEnumeratorNameAsString` (`self.ElementalType`))))
  (`TextRenderComponent.K2_SetText` (`self.TextElemType`) (`KismetTextLibrary.Conv_StringToText` (`|GetEnumeratorNameAsString` (`self.WeaponType`))))
  (`TextRenderComponent.K2_SetText` (`self.TextDmgType`) (`KismetTextLibrary.Conv_StringToText` (`KismetStringLibrary.Concat_StrStr` (`KismetStringLibrary.Conv_IntToString` (`self.MinDamage`)) "-" (`KismetStringLibrary.Conv_IntToString` (`self.MaxDamage`))))))

(fn `UserConstructionScript`)