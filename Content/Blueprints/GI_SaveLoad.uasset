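; Game instance Blueprint that saves and loads player progress through an SG_Coding2 save object in a named slot.
; SaveGame reuses or creates the save, then writes the character's stamina, transform, sprint and shoot flags.
; LoadGame teleports the character to the saved transform and copies saved stamina into a Stamina variable.
; On load, sprint and shoot flags copy from character to save object rather than being restored, and PlayerRespawn is assigned to itself.
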(event `SaveGame`
  (`KismetSystemLibrary.PrintString` "Starting Save Game")
  (bind _returnvalue (`GameplayStatics.DoesSaveGameExist` (`self.Slot Name`))) ; Have we already saved before?
  (if _returnvalue
    (bind _returnvalue_2 (`GameplayStatics.LoadGameFromSlot` (`self.Slot Name`))) ; Load our previous save file
    (set `self.Saver Subclass` _returnvalue_2)
    (else
      (bind _returnvalue_3 (`GameplayStatics.CreateSaveGameObject` "/Game/Blueprints/SG_Coding2.SG_Coding2_C")) ; Create a new save file
      (set `self.Saver Subclass` _returnvalue_3)))
  ;[0.474 0.2787 0.1273] Save Game Data
  (bind _assg_coding_2 (cast `/Game/Blueprints/SG_Coding2` (`self.Saver Subclass`)))
  ;[0.1032 0.3385 0.06808] Player's Current Data
  (bind _asbp_third_person_character (cast `/Game/ThirdPerson/Blueprints/BP_ThirdPersonCharacter` (`GameplayStatics.GetPlayerCharacter` 0)))
  (set `/Game/Blueprints/SG_Coding2.PlayerStamina` (`/Game/ThirdPerson/Blueprints/BP_ThirdPersonCharacter.Stamina` _asbp_third_person_character) _assg_coding_2)
  (set `/Game/Blueprints/SG_Coding2.PlayerTransform` (`SceneComponent.K2_GetComponentToWorld` (`Character.CapsuleComponent` _asbp_third_person_character)) _assg_coding_2)
  (set `/Game/Blueprints/SG_Coding2.PlayerCanSprint` (`/Game/ThirdPerson/Blueprints/BP_ThirdPersonCharacter.CanSprint` _asbp_third_person_character) _assg_coding_2)
  (set `/Game/Blueprints/SG_Coding2.PlayerCanShoot` (`/Game/ThirdPerson/Blueprints/BP_ThirdPersonCharacter.CanShoot` _asbp_third_person_character) _assg_coding_2)
  (`GameplayStatics.SaveGameToSlot` (`self.Saver Subclass`) (`self.Slot Name`))
  (`KismetSystemLibrary.PrintString` "Game is successfully saved" true true (struct :`G` 1.0 :`B` 0.253745 :`A` 1.0)))

(event `LoadGame`
  (`KismetSystemLibrary.PrintString` "Starting Load Game")
  (bind _returnvalue (`GameplayStatics.DoesSaveGameExist` (`self.Slot Name`)))
  (if _returnvalue
    (bind _returnvalue_2 (`GameplayStatics.LoadGameFromSlot` (`self.Slot Name`)))
    ;[0.4167 0.5472 1] Load Game
    (bind _asbp_third_person_character (cast `/Game/ThirdPerson/Blueprints/BP_ThirdPersonCharacter` (`GameplayStatics.GetPlayerCharacter` 0)))
    (bind _assg_coding_2 (cast `/Game/Blueprints/SG_Coding2` _returnvalue_2))
    (set `self.Saver Subclass` _assg_coding_2)
    (set `self.Stamina` (`/Game/Blueprints/SG_Coding2.PlayerStamina` _assg_coding_2))
    (`Actor.K2_SetActorTransform` _asbp_third_person_character (`/Game/Blueprints/SG_Coding2.PlayerTransform` _assg_coding_2) false true)
    (set `/Game/Blueprints/SG_Coding2.PlayerRespawn` (`/Game/Blueprints/SG_Coding2.PlayerRespawn` _assg_coding_2) _assg_coding_2)
    (set `/Game/Blueprints/SG_Coding2.PlayerCanSprint` (`/Game/ThirdPerson/Blueprints/BP_ThirdPersonCharacter.CanSprint` _asbp_third_person_character) _assg_coding_2)
    (set `/Game/Blueprints/SG_Coding2.PlayerCanShoot` (`/Game/ThirdPerson/Blueprints/BP_ThirdPersonCharacter.CanShoot` _asbp_third_person_character) _assg_coding_2)))