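; Game mode that gives each level its own save, keeping collected coins, door states and the player's checkpoint position.
; On BeginPlay it loads or creates an SG_LevelSAVE in a slot named after the current level, then restores coins, doors and any non-zero player location.
; Checkpoint stores the player transform and saves to that slot.
; FinishedLevel clears the transform and saves, so the stored position is not reused.
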(event `self.ReceiveBeginPlay`
  (bind _levelsave (`self.LevelSAVE`))
  (bind _playertransform_location (`KismetMathLibrary.BreakTransform` (`/Game/Blueprints/NewSaves/SG_LevelSAVE.PlayerTransform` _levelsave)))
  (`KismetSystemLibrary.PrintString` "LOADED into GM_2Coding Game Mode" true true (struct :`R` 0.510417 :`G` 0.338 :`A` 1.0))
  ;[1 1 1] Is there a level save file for this level's name?
  ; If not, create one, so that we can start editing it.
  ; If there is, load it and store it to the "Level SAVE" variable, so we can start editing it.
  (bind _returnvalue (`GameplayStatics.GetCurrentLevelName` true))
  (bind _returnvalue_2 (`GameplayStatics.DoesSaveGameExist` _returnvalue))
  (if _returnvalue_2
    (bind _returnvalue_3 (`GameplayStatics.LoadGameFromSlot` _returnvalue))
    (bind _assg_level_save (cast `/Game/Blueprints/NewSaves/SG_LevelSAVE` _returnvalue_3))
    (bind _output_get (set `self.LevelSAVE` _assg_level_save))
    (`/Game/Blueprints/NewSaves/SG_LevelSAVE.LoadCollectedCoins` _output_get) ; Change the coins that have already been collected
    (`/Game/Blueprints/NewSaves/SG_LevelSAVE.NEWLoadDoorStates` _output_get)
    (if (not (`KismetMathLibrary.EqualExactly_VectorVector` _playertransform_location))
      (`SceneComponent.K2_SetWorldTransform` (`Character.CapsuleComponent` (`GameplayStatics.GetPlayerCharacter` 0)) (`/Game/Blueprints/NewSaves/SG_LevelSAVE.PlayerTransform` _levelsave) false false))
    (else
      (bind _returnvalue_4 (`GameplayStatics.CreateSaveGameObject` "/Game/Blueprints/NewSaves/SG_LevelSAVE.SG_LevelSAVE_C"))
      (set `self.LevelSAVE` _returnvalue_4))))

(event `Save Game`
  (bind _returnvalue (`GameplayStatics.GetCurrentLevelName` true))
  (bind _returnvalue_2 (`GameplayStatics.SaveGameToSlot` (`self.LevelSAVE`) _returnvalue))
  (if _returnvalue_2
    (`KismetSystemLibrary.PrintString` "SAVED LEVEL" true true (struct :`R` 0.118773 :`G` 1.0 :`A` 1.0))
    (else
      (`KismetSystemLibrary.PrintString` "COULD NOT SAVE LEVEL" true true (struct :`R` 0.380208 :`B` 0.007334 :`A` 1.0)))))

(fn `Checkpoint`
  (params (PlayerTransform :type "Transform Structure"))
  (set `/Game/Blueprints/NewSaves/SG_LevelSAVE.PlayerTransform` PlayerTransform (`self.LevelSAVE`))
  (`self.Save Game`))

(fn `FinishedLevel`
  (set `/Game/Blueprints/NewSaves/SG_LevelSAVE.PlayerTransform` (struct) (`self.LevelSAVE`)) ; Restart player start location to 0, 0, 0
  (`self.Save Game`))

(fn `UserConstructionScript`)