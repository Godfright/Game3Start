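; Save game Blueprint, going by its SG_ prefix, that restores collected coin and door states on load.
; LoadCollectedCoins prints a debug message, then calls LoadCollectedState on each valid coin in CollectedCoins.
; NEWLoadDoorStates, replacing a LoadDoorStates made in the wrong Blueprint, calls QuietOpen on valid loop elements.
; It checks that NEWOpenDoors is non-empty, but its loop shows no connected array.
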(fn `LoadCollectedCoins`
  (bind _collectedcoins (`self.CollectedCoins`))
  (`KismetSystemLibrary.PrintString` null "Load Collected Coins START")
  (if (> (`KismetArrayLibrary.Array_Length` _collectedcoins) 0)
    (for _array_element _collectedcoins
      (`/Engine/EditorBlueprintResources/StandardMacros.IsValid` _array_element
        (:`Is Valid`
          (`/Game/Blueprints/BP_Coin.Load Collected State` _array_element))))))

(fn `NEWLoadDoorStates`
  (if (> (`KismetArrayLibrary.Array_Length` (`self.NEWOpenDoors`)) 0)
    (for _array_element _
      (`/Engine/EditorBlueprintResources/StandardMacros.IsValid` _array_element
        (:`Is Valid`
          (`/Game/Blueprints/BP_CameraDoor.quietOpen` _array_element))))))