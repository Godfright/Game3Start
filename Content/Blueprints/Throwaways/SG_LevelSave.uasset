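; SG_LevelSave is a level save, likely a SaveGame object, for restoring collected objects and door states.
; LoadCollectedObjects loops over CollectedObjects and calls LoadCollectedState on each valid entry.
; LoadDoorStates is unfinished: it checks that OpenDoors is non-empty, but its loop has no array wired in and does nothing after the validity check.
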(fn `LoadCollectedObjects`
  (bind _collectedobjects (`self.CollectedObjects`))
  (if (> (`KismetArrayLibrary.Array_Length` _collectedobjects) 0)
    (for _array_element _collectedobjects
      (`/Engine/EditorBlueprintResources/StandardMacros.IsValid` _array_element
        (:`Is Valid`
          (`/Game/Blueprints/BP_Coin.Load Collected State` _array_element))))))

(fn `LoadDoorStates`
  (if true
    (if (> (`KismetArrayLibrary.Array_Length` (`self.OpenDoors`)) 0)
      (for _array_element _
        (`/Engine/EditorBlueprintResources/StandardMacros.IsValid` _array_element)))))